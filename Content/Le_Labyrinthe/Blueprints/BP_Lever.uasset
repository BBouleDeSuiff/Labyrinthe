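; BP_Lever is a two-state lever for the labyrinth that shows its on or off position by swapping two cylinder meshes.
; BeginPlay starts it off, with CylinderOff visible and CylinderOn hidden.
; The ToggleLever event flips the IsOn flag and the visibility of both cylinders, reusing the BeginPlay logic to switch off.
; The Blueprint itself only changes this state and does not trigger other actors.
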(event Custom|ToggleLever
  (bind _cylinderon (Variables|Default|GetCylinderOn))
  (if (Variables|Default|GetIsOn)
    (Development|SetHiddeninGame _cylinderon true false)
    (Development|SetHiddeninGame (Variables|Default|GetCylinderOff) false false)
    (Variables|Default|SetIsOn false)
    (else
      (Development|SetHiddeninGame _cylinderon false false)
      (Development|SetHiddeninGame (Variables|Default|GetCylinderOff) true false)
      (Variables|Default|SetIsOn true))))

(event EventBeginPlay
  (Development|SetHiddeninGame (Variables|Default|GetCylinderOn) true false)
  (Development|SetHiddeninGame (Variables|Default|GetCylinderOff) false false)
  (Variables|Default|SetIsOn false))

(fn ConstructionScript)